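; Interactable door that swings open and closed, with an optional item-based lock and an option to start open.
; An inventory check on BP_FirstPersonCharacter unlocks it, optionally consuming the items, and later interactions toggle it.
; A FlipFlop plays or reverses a timeline driving door yaw and switches the look-at action name.
; IsPlayerCharacterInteractable selects whether the player or only other actors can trigger it.
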(event EventInteract
  (params (ActorTriggeringInteract :type Actor%20Object%20Reference))
  (bind _isplayercharacterinteractable (Variables|Default|GetisPlayerCharacterInteractable))
  (bind _asbp_first_person_character (Utilities|Casting|CastToBP_FirstPersonCharacter ActorTriggeringInteract)
    (:then
      (if _isplayercharacterinteractable
        (if (Variables|Default|GetisItemNeeded) :!label _label
          (if (.ReturnValue (Utilities|Map|Find (Variables|/Game/FirstPerson/Blueprints/BP_FirstPersonCharacter.BP_FirstPersonCharacter_C|GetInventory _asbp_first_person_character) (Variables|Default|GetItemID)))
            (if (>= (.Value (Utilities|Map|Find (Variables|/Game/FirstPerson/Blueprints/BP_FirstPersonCharacter.BP_FirstPersonCharacter_C|GetInventory _asbp_first_person_character) (Variables|Default|GetItemID))) (Variables|Default|GetAmountOfItemsNeeded))
              (Variables|Default|SetisItemNeeded false)
              (Audio|PlaySound2D "/Game/Images/Narra/lock-the-door-46014.lock-the-door-46014" 1.0 1.0 0.0 0 0)
              (Development|PrintString "Imaginez un son d'unlock")
              (if (Variables|Default|GetisItemRemoved)
                (Utilities|Map|Add (Variables|/Game/FirstPerson/Blueprints/BP_FirstPersonCharacter.BP_FirstPersonCharacter_C|GetInventory _asbp_first_person_character) (Variables|Default|GetItemID) (- (.Value (Utilities|Map|Find (Variables|/Game/FirstPerson/Blueprints/BP_FirstPersonCharacter.BP_FirstPersonCharacter_C|GetInventory _asbp_first_person_character) (Variables|Default|GetItemID))) (Variables|Default|GetAmountOfItemsNeeded))))
              (if (stale _isa)
                (Variables|Default|SetLookAtActionName (Variables|Default|GetActionNameForA))
                (else
                  (Variables|Default|SetLookAtActionName (Variables|Default|GetActionNameForB))))))
          (else
            (bind _isa (Utilities|FlowControl|FlipFlop)
              (:A
                (Variables|Default|SetLookAtActionName (Variables|Default|GetActionNameForA))
                (bind _newangle (Timeline|TL_MoveDoor Play)
                  (:Update
                    (Audio|PlaySound2D "/Game/Images/Narra/open-door-stock-sfx-454246.open-door-stock-sfx-454246" 1.0 1.0 0.0 0 0)
                    (Transformation|SetRelativeRotation (Variables|Default|GetDoor) (Math|Rotator|MakeRotator 0.0 0.0 _newangle) false false))))
              (:B
                (Variables|Default|SetLookAtActionName (Variables|Default|GetActionNameForB))
                (Timeline|TL_MoveDoor Reverse)))))))
    (:CastFailed
      (if (not _isplayercharacterinteractable)
        (goto _label)))))

(event EventBeginPlay
  (if (Variables|Default|GetisOpenedAtStart)
    (bind _isa (Utilities|FlowControl|FlipFlop)
      (:A
        (Variables|Default|SetLookAtActionName (Variables|Default|GetActionNameForA))
        (bind _newangle (Timeline|TL_MoveDoor Play)
          (:Update
            (Audio|PlaySound2D "/Game/Images/Narra/open-door-stock-sfx-454246.open-door-stock-sfx-454246" 1.0 1.0 0.0 0 0)
            (Transformation|SetRelativeRotation (Variables|Default|GetDoor) (Math|Rotator|MakeRotator 0.0 0.0 _newangle) false false))))
      (:B
        (Variables|Default|SetLookAtActionName (Variables|Default|GetActionNameForB))
        (Timeline|TL_MoveDoor Reverse)))))

(fn ConstructionScript
  (|CallParentFunction))