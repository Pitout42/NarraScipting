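; Inspectable Rubik's cube prop that the player picks up to examine, then returns to where it was.
; Interact swaps input from the first-person character to this actor and snaps it to the character's inspection component.
; While inspecting, mouse look rotates the object.
; The interact input action detaches it, restores its starting transform saved at BeginPlay and gives input back to the player.
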(event Input|EnhancedActionEvents|EnhancedInputActionIA_Interact
  (params (ActionValue :type Boolean) (ElapsedSeconds :type Float%20%28double-precision%29) (TriggeredSeconds :type Float%20%28double-precision%29) (InputAction :type Input%20Action%20Object%20Reference :default "/Game/Input/Actions/IA_Interact.IA_Interact"))
  (CallFunction|StopInspection))

(event Input|EnhancedActionEvents|EnhancedInputActionIA_Look
  (params (ActionValue :type Vector%202D%20Structure) (ElapsedSeconds :type Float%20%28double-precision%29) (TriggeredSeconds :type Float%20%28double-precision%29) (InputAction :type Input%20Action%20Object%20Reference :default "/Game/Input/Actions/IA_Look.IA_Look")))

(event Input|EnhancedActionEvents|EnhancedInputActionIA_MouseLook
  (params (ActionValue :type Vector%202D%20Structure) (ElapsedSeconds :type Float%20%28double-precision%29) (TriggeredSeconds :type Float%20%28double-precision%29) (InputAction :type Input%20Action%20Object%20Reference :default "/Game/Input/Actions/IA_MouseLook.IA_MouseLook"))
  (bind (_x _y) (Math|Vector2D|BreakVector2D ActionValue))
  (Transformation|SetActorRotation (Math|Rotator|CombineRotators (Transformation|GetActorRotation) (Math|Rotator|MakeRotator 0.0 (* _y 3.0) (* _x -3.0)))))

(event EventBeginPlay
  (Variables|Default|SetInitLocation (Transformation|GetActorLocation))
  (Variables|Default|SetInitRotation (Transformation|GetActorRotation)))

(event Collision|EventActorBeginOverlap
  (params (OtherActor :type Actor%20Object%20Reference)))

(event EventTick
  (params (DeltaSeconds :type Float%20%28single-precision%29)))

(event EventInteract
  (params (ActorTriggeringInteract :type Actor%20Object%20Reference))
  (bind _asbp_first_person_character (Utilities|Casting|CastToBP_FirstPersonCharacter ActorTriggeringInteract))
  (Variables|Default|SetPlayerBP _asbp_first_person_character)
  (CallFunction|StartInspection))

(fn ConstructionScript
  (|CallParentFunction))

(fn StartInspection
  (bind _returnvalue (Game|GetPlayerController 0))
  (bind _playerbp (Variables|Default|GetPlayerBP))
  (Input|DisableInput _playerbp _returnvalue)
  (Input|EnableInput _returnvalue)
  (Transformation|AttachComponentToComponent (Variables|/Game/FirstPerson/Blueprints/BP_FirstPersonCharacter.BP_FirstPersonCharacter_C|GetItemInspecrt _playerbp) "" "SnapToTarget" "SnapToTarget" "SnapToTarget" true))

(fn StopInspection
  (bind _returnvalue (Game|GetPlayerController 0))
  (Input|DisableInput _returnvalue)
  (Input|EnableInput (Variables|Default|GetPlayerBP) _returnvalue)
  (Transformation|DetachFromActor "KeepRelative" "KeepRelative" "KeepRelative")
  (Transformation|SetActorLocationAndRotation (Variables|Default|GetInitLocation) (Variables|Default|GetInitRotation)))