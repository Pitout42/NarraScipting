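; BP_Inspectable is an actor the first-person character can interact with to begin an inspection.
; On BeginPlay it caches its location and the forward (X) vector of its rotation.
; Interact casts the triggering actor to BP_FirstPersonCharacter, stores it as PlayerBP and calls StartInspection.
; StartInspection and StopInspection are empty here, so no inspection behavior is implemented in this Blueprint.
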(event EventBeginPlay
  (Variables|Default|SetInitLocation (Transformation|GetActorLocation))
  (Variables|Default|SetInitRotation (Math|Rotator|GetRotationXVector (Transformation|GetActorRotation))))

(event Collision|EventActorBeginOverlap
  (params (OtherActor :type Actor%20Object%20Reference)))

(event EventTick
  (params (DeltaSeconds :type Float%20%28single-precision%29)))

(event EventInteract
  (params (ActorTriggeringInteract :type Actor%20Object%20Reference))
  (bind _asbp_first_person_character (Utilities|Casting|CastToBP_FirstPersonCharacter ActorTriggeringInteract))
  (Variables|Default|SetPlayerBP _asbp_first_person_character)
  (CallFunction|StartInspection))

(fn ConstructionScript
  (|CallParentFunction))

(fn StartInspection)

(fn StopInspection)