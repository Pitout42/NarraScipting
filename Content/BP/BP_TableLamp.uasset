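; BP_TableLamp is an interactable table lamp whose two spotlights switch on and off with a click sound.
; Interact can first require an inventory item from the first-person character, optionally consuming it, with an unlock sound and placeholder debug print.
; Once unlocked, a FlipFlop alternates the look-at action name while visibility toggles.
; BeginPlay toggles the lights from their default state, then reruns the switch path if IsOpenAtStart.
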(event EventInteract
  (params (ActorTriggeringInteract :type Actor%20Object%20Reference))
  (bind _isplayercharacterinteractable (Variables|Default|GetisPlayerCharacterInteractable))
  (bind _asbp_first_person_character (Utilities|Casting|CastToBP_FirstPersonCharacter ActorTriggeringInteract)
    (:then
      (if _isplayercharacterinteractable
        (if (Variables|Default|GetIs%20item%20need) :!label _label
          (if (.ReturnValue (Utilities|Map|Find (Variables|/Game/FirstPerson/Blueprints/BP_FirstPersonCharacter.BP_FirstPersonCharacter_C|GetInventory _asbp_first_person_character) (Variables|Default|GetItem%20ID)))
            (if (>= (.Value (Utilities|Map|Find (Variables|/Game/FirstPerson/Blueprints/BP_FirstPersonCharacter.BP_FirstPersonCharacter_C|GetInventory _asbp_first_person_character) (Variables|Default|GetItem%20ID))) (Variables|Default|GetAmount%20need))
              (Variables|Default|SetIs%20item%20need false)
              (Audio|PlaySound2D "/Game/Images/Narra/bottle-screw-85702.bottle-screw-85702" 1.0 1.0 0.0 0 0)
              (Development|PrintString "Imaginez un son d'unlock")
              (if (Variables|Default|Getis%20item%20removed)
                (Utilities|Map|Add (Variables|/Game/FirstPerson/Blueprints/BP_FirstPersonCharacter.BP_FirstPersonCharacter_C|GetInventory _asbp_first_person_character) (Variables|Default|GetItem%20ID) (- (.Value (Utilities|Map|Find (Variables|/Game/FirstPerson/Blueprints/BP_FirstPersonCharacter.BP_FirstPersonCharacter_C|GetInventory _asbp_first_person_character) (Variables|Default|GetItem%20ID))) (Variables|Default|GetAmount%20need))))
              (if (stale _isa)
                (Variables|Default|SetLookAtActionName (Variables|Default|GetAction%20Name%20For%20A))
                (else
                  (Variables|Default|SetLookAtActionName (Variables|Default|GetAction%20Name%20For%20B))))))
          (else
            (bind _isa (Utilities|FlowControl|FlipFlop)
              (:A
                (Variables|Default|SetLookAtActionName (Variables|Default|GetAction%20Name%20For%20A)))
              (:B
                (Variables|Default|SetLookAtActionName (Variables|Default|GetAction%20Name%20For%20B))))
            (Audio|PlaySound2D "/Game/Images/Narra/light-switch-382712.light-switch-382712" 1.0 1.0 0.0 0 0)
            (Rendering|ToggleVisibility (Variables|Default|GetSpotLight) false)))))
    (:CastFailed
      (if _isplayercharacterinteractable
        (goto _label)))))

(event EventBeginPlay
  (Rendering|ToggleVisibility (Variables|Default|GetSpotLight) false)
  (if (Variables|Default|GetIs%20open%20at%20start)
    (bind _isa (Utilities|FlowControl|FlipFlop)
      (:A
        (Variables|Default|SetLookAtActionName (Variables|Default|GetAction%20Name%20For%20A)))
      (:B
        (Variables|Default|SetLookAtActionName (Variables|Default|GetAction%20Name%20For%20B))))
    (Audio|PlaySound2D "/Game/Images/Narra/light-switch-382712.light-switch-382712" 1.0 1.0 0.0 0 0)
    (Rendering|ToggleVisibility (Variables|Default|GetSpotLight) false)))

(fn ConstructionScript
  (|CallParentFunction))